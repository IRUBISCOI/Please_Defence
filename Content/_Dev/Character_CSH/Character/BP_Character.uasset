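; Player character Blueprint, in a developer folder, that links a weapon enhancement UI to the character's weapon damage.
; On BeginPlay it runs the parent logic, creates the Enhancement_Weapon widget, adds it to the viewport and binds its ApplyDamage event.
; When that event fires, it passes the widget's WeaponDamage to SetWeaponDamage.
; An unconnected graph for spawning BP_Weapon on the mesh's weapon socket never runs.
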(event `self.ReceiveBeginPlay`
  (`parent.ReceiveBeginPlay`)
  (bind _returnvalue (`|CreateWidget` "/Game/_Dev/Character_CSH/UI/Enhancement_Weapon.Enhancement_Weapon_C" (`GameplayStatics.GetPlayerController` 0)))
  (bind _output_get (set `self.Enhancement_UI` _returnvalue))
  (`UserWidget.AddToViewport` _output_get 0)
  (add `/Game/_Dev/Character_CSH/UI/Enhancement_Weapon.Apply_Damage` _output_get (delegate `ApplyDamage`)))

(event `ApplyDamage`
  (`self.Set_Weapon_Damage` (`/Game/_Dev/Character_CSH/UI/Enhancement_Weapon.Weapon_Damage` (stale `self.ReceiveBeginPlay` _output_get))))

(fn `UserConstructionScript`)