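; Player state Blueprint that links gold and weapon damage to the in-game HUD and the weapon enhancement screen.
; BeginPlay creates both widgets, caches an EnhancementResult actor and sets starting gold; overridden setters push changes to both widgets.
; Enhancement results feed the HUD's calculation, whose damage event writes back weapon damage.
; Show/hide events toggle cursor and input mode; viewport attachment and enhancement binding happen only when showing finds no valid widget.
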(event `self.ReceiveBeginPlay`
  (`|ExecutionSequence`
    (:`then_0`
      (bind _returnvalue (`|CreateWidget` "/Game/_Dev/Character_CSH/UI/IngameUI.IngameUI_C" (`GameplayStatics.GetPlayerController` 0)))
      (bind _output_get (set `self.IngameUI` _returnvalue))
      (set `/Game/_Dev/Character_CSH/UI/IngameUI.Owning_Gold` (`self.Get_Gold`) _output_get)
      (`UserWidget.AddToViewport` _output_get 0)
      (add `/Game/_Dev/Character_CSH/UI/IngameUI.Apply_Damage` _output_get (delegate `ApplyWeaponDamage`)))
    (:`then_1`
      (bind _outactors (`GameplayStatics.GetAllActorsOfClass` "/Game/_Dev/Character_CSH/UI/Enhancement_Image/EnhancementResult.EnhancementResult_C"))
      (for _array_element _outactors
        (set `self.Enhancement Display` _array_element)))
    (:`then_2`
      (bind _returnvalue_2 (`|CreateWidget` "/Game/_Dev/Character_CSH/UI/Enhancement_Display.Enhancement_Display_C" (`GameplayStatics.GetPlayerController` 0)))
      (bind _output_get_2 (set `self.EnhancementUI` _returnvalue_2))
      (set `/Game/_Dev/Character_CSH/UI/Enhancement_Display.Owning_Gold` (`self.Get_Gold`) _output_get_2)
      (`self.Set_Gold` 1000))))

(event `ApplyWeaponDamage`
  (`self.Set_Weapon_Damage` (`/Game/_Dev/Character_CSH/UI/IngameUI.Weapon_Damage` (stale `self.ReceiveBeginPlay` _output_get))))

(event `self.UI_AmmoUpdate`
  (set `/Game/_Dev/Character_CSH/UI/IngameUI.Ammo` (`self.Ammo`) (`self.IngameUI`)))

(event `EnhancementUI_On`
  (bind _returnvalue (`GameplayStatics.GetPlayerController` 0))
  (bind _enhancementui (`self.EnhancementUI`))
  (`/Engine/EditorBlueprintResources/StandardMacros.IsValid` _enhancementui
    (:`Is Valid`
      (`Widget.SetVisibility` _enhancementui "Visible"))
    (:`Is Not Valid`
      (bind _returnvalue_2 (`|CreateWidget` "/Game/_Dev/Character_CSH/UI/Enhancement_Display.Enhancement_Display_C" (`GameplayStatics.GetPlayerController` 0)))
      (bind _output_get (set `self.EnhancementUI` _returnvalue_2))
      (set `/Game/_Dev/Character_CSH/UI/Enhancement_Display.Owning_Gold` (`self.Get_Gold`) (`self.EnhancementUI`))
      (`UserWidget.AddToViewport` _output_get 0)
      (set `/Game/_Dev/Character_CSH/UI/Enhancement_Display.EnhancementDisplay` (`self.Enhancement Display`) _output_get)
      (add `/Game/_Dev/Character_CSH/UI/Enhancement_Display.Apply_Enhancement` _output_get (delegate `ApplyEnhancement`))))
  (set `PlayerController.bShowMouseCursor` true _returnvalue)
  (`WidgetBlueprintLibrary.SetInputMode_GameAndUIEx` _returnvalue null))

(event `ApplyEnhancement`
  (bind _enhancementui (`self.EnhancementUI`))
  (`/Game/_Dev/Character_CSH/UI/IngameUI.CalEnhance` (`self.IngameUI`) (`/Game/_Dev/Character_CSH/UI/Enhancement_Display.Enhancement_Ratio` _enhancementui) (`/Game/_Dev/Character_CSH/UI/Enhancement_Display.Enhancement_Level` _enhancementui) (`/Game/_Dev/Character_CSH/UI/Enhancement_Display.Weapon_Damage` _enhancementui) (`/Game/_Dev/Character_CSH/UI/Enhancement_Display.Enhancement_Cost` _enhancementui) (`/Game/_Dev/Character_CSH/UI/Enhancement_Display.Owning_Gold` _enhancementui)))

(event `EnhancementUI_Off`
  (bind _returnvalue (`GameplayStatics.GetPlayerController` 0))
  (`Widget.SetVisibility` (`self.EnhancementUI`) "Collapsed")
  (set `PlayerController.bShowMouseCursor` false _returnvalue)
  (`WidgetBlueprintLibrary.SetInputMode_GameOnly` _returnvalue))

(event `self.Set_Gold`
  (params (newGold :type Integer))
  (`parent.Set_Gold` newGold)
  (bind _output_get (set `/Game/_Dev/Character_CSH/UI/IngameUI.Owning_Gold` newGold (`self.IngameUI`)))
  (set `/Game/_Dev/Character_CSH/UI/Enhancement_Display.Owning_Gold` _output_get (`self.EnhancementUI`)))

(event `self.Set_Weapon_Damage`
  (params (Damage :type Integer))
  (bind _enhancementui (`self.EnhancementUI`))
  (`parent.Set_Weapon_Damage` Damage)
  (bind _output_get (set `/Game/_Dev/Character_CSH/UI/IngameUI.Weapon_Damage` Damage (`self.IngameUI`)))
  (bind _output_get_2 (set `/Game/_Dev/Character_CSH/UI/Enhancement_Display.Weapon_Damage` _output_get _enhancementui))
  (`/Game/_Dev/Character_CSH/UI/Enhancement_Display.CalNextWeaponDamage` _enhancementui _output_get_2))

(fn `UserConstructionScript`)