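; Development monster actor that travels along the level's BP_Spline and is destroyed when damage depletes its HP.
; BeginPlay finds the spline and sets HP from a scaled DT_Max table value.
; FollowSpline snaps to a spline point, registers in BPSpawn's monster array, then a speed-scaled timeline drives position and rotation along the path.
; SetVisibleLocation sets visibility, removes spawner array entries and calls FollowSpline; some nodes are left disconnected.
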(event `self.ReceiveBeginPlay`
  ;[1 1 1] 스플라인
  (`self.SetMax`)
  (bind _returnvalue (`GameplayStatics.GetActorOfClass` "/Game/_Dev/Monster_KHJ/BP_Spline.BP_Spline_C"))
  (set `self.BP_Spline` _returnvalue)
  (set `self.MonsterCurHP` (`self.MonsterMaxHP`)))

(event `FollowSpline`
  (bind _spline (`/Game/_Dev/Monster_KHJ/BP_Spline.Spline` (`self.BP_Spline`)))
  ;[1 1 1] 초기값 리셋
  (bind (_sweephitresult _returnvalue) (`self.K2_SetActorLocation` (`SplineComponent.GetLocationAtSplinePoint` (`/Game/_Dev/Monster_KHJ/BP_Spline.Spline` (`self.BP_Spline`)) 35 "World")))
  (`SceneComponent.SetVisibility` (`self.Capsule`) _returnvalue false)
  (`SceneComponent.SetVisibility` (`self.SkeletalMesh`) _returnvalue false)
  (`KismetArrayLibrary.Array_Add` (`/Game/_Dev/Monster_KHJ/BP_Spawn.MonArray` (`self.BP_Spawn`)))
  ;[1 1 1] 스플라인상 움직임
  (`TimelineComponent.SetPlayRate` (`self.Move`) (`self.MonMoveSpeed`))
  (bind (_direction `_새_트랙_0`) (`Timeline|Move` :!via `PlayFromStart`)
    (:`Update`
      (bind _returnvalue_2 (`KismetMathLibrary.Lerp` 0.0 (`SplineComponent.GetSplineLength` (`/Game/_Dev/Monster_KHJ/BP_Spline.Spline` (`self.BP_Spline`))) `_새_트랙_0`))
      (`self.K2_SetActorTransform` (`KismetMathLibrary.MakeTransform` (`SplineComponent.GetLocationAtDistanceAlongSpline` _spline _returnvalue_2 "World") (`SplineComponent.GetRotationAtDistanceAlongSpline` _spline _returnvalue_2 "World"))))))

(event `SetVisibleLocation`
  (bind _bp_spawn (`self.BP_Spawn`))
  ;[1 1 1] Off Visibility & Location
  (`SceneComponent.SetVisibility` (`self.Capsule`) (`self.Visible`) false)
  (`SceneComponent.SetVisibility` (`self.SkeletalMesh`) (`self.Visible`) false)
  (for _index (range (+ (`KismetArrayLibrary.Array_Length` (`/Game/_Dev/Monster_KHJ/BP_Spawn.MonArrayNum` _bp_spawn)) 1))
    (`KismetArrayLibrary.Array_Remove` (`/Game/_Dev/Monster_KHJ/BP_Spawn.MonArray` _bp_spawn) _index)
    (`self.FollowSpline`)))

(fn `MonsterDie`
  (`self.K2_DestroyActor`))

(fn `OnApplyDamage`
  (params (Damage :type "Float (double-precision)"))
  (if (> (`self.MonsterCurHP`) 0.0)
    (set `self.MonsterCurHP` (- (`self.MonsterCurHP`) Damage))
    (if (<= (`self.MonsterCurHP`) 0.0)
      (`self.MonsterDie`))))

(fn `SetMax`
  (bind _returnvalue (`|GetDataTableRow` "/Game/_Dev/Monster_KHJ/DT_Max.DT_Max" "NewRow")
    (:`then`
      (bind _structout (setmembers `/Game/_Dev/Monster_KHJ/ST_Max` :`StructRef` _returnvalue))
      (set `self.MonsterMaxHP` (* (break `/Game/_Dev/Monster_KHJ/ST_Max` _structout) 1.25)))))

(fn `UserConstructionScript`)