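; BP_Spawn is a monster spawner that creates BP_Monster actors at its Arrow.
; After a start delay, Tick consumes GameState's SpawnTimeBoolean for each spawn and records the monster in two arrays.
; Spawning stops at a hard-coded array limit or the data table's MonsterMaxCount, setting a flag for either case.
; PoolingRemove only removes monsters from MonArrayNum, and the bound data table update only prints its values.
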(event `Update`
  (params (MaxHP :type "Float (double-precision)") (MaxCount :type "Float (double-precision)") (Speed :type "Float (double-precision)"))
  ;[1 1 1] Update Value
  (`KismetSystemLibrary.PrintString` (`KismetStringLibrary.Concat_StrStr` (`KismetStringLibrary.Conv_DoubleToString` MaxHP) "   " (`KismetStringLibrary.Conv_DoubleToString` MaxCount) "   " (`KismetStringLibrary.Conv_DoubleToString` Speed) "   " "Spawn Bind DT") true true (struct :`R` 1.0 :`G` 0.098822 :`A` 1.0) 2222.0))

(event `self.ReceiveBeginPlay`
  (`KismetSystemLibrary.Delay` 0.1)
  (bind _asbp_game_state (cast `/Game/_Dev/Monster_KHJ/BP_GameState` (`GameplayStatics.GetGameState`)))
  (set `self.BP_GameState` _asbp_game_state)
  ;[1 1 1] Update Value
  (add `/Game/_Dev/Monster_KHJ/BP_GameState.UpdateDT` (`self.BP_GameState`) (delegate `Update`)))

(event `self.ReceiveTick`
  (params (DeltaSeconds :type "Float (single-precision)"))
  (bind _spawncount (`self.SpawnCount`))
  (bind _bp_gamestate (`self.BP_GameState`))
  (bind (_maindt_stage _maindt_monstermaxhp _maindt_monstermaxcount) (break `/Game/_Dev/Monster_KHJ/ST_Max` (`/Game/_Dev/Monster_KHJ/BP_GameState.MainDT` (`self.BP_GameState`))))
  ;[1 1 1] Start Dealy
  (bind _output_get (set `self.StartDelayTime_Cur` (+ DeltaSeconds (`self.StartDelayTime_Cur`))))
  (if (> _output_get (`self.StartDelayTime_Del`))
    (if (`self.MaxArrayCount`)
      (set `self.MaxArraySpawning` true)
      (elif (`self.MonArrayEqualDT`)
        (set `self.EqualDTSpawning` true)
        (elif (`/Game/_Dev/Monster_KHJ/BP_GameState.SpawnTimeBoolean` _bp_gamestate)
          (set `/Game/_Dev/Monster_KHJ/BP_GameState.SpawnTimeBoolean` false _bp_gamestate)
          (bind _outputpin (`self.SpawnNumber`))
          ;[1 1 1] Add Array
          (bind _returnvalue (`KismetArrayLibrary.Array_Add` (`self.MonArray`) _outputpin))
          (`KismetArrayLibrary.Array_Add` (`self.MonArrayNum`) _outputpin)
          (set `self.SpawnCount` (+ (`self.SpawnCount`) 1.0))
          ;[1 1 1] Max Array Count
          (set `self.MaxArrayCount` (>= _returnvalue 8))
          ;[1 1 1] MonArray Equal DT
          (set `self.MonArrayEqualDT` (>= _spawncount _maindt_monstermaxcount))
          (`KismetSystemLibrary.PrintString` (`KismetStringLibrary.Conv_DoubleToString` _spawncount)))))))

(event `Pooling Remove`
  (params (ItemToFind :type "/Game/_Dev/Monster_KHJ/BP_Monster Object Reference (by ref)"))
  (bind _monarraynum (`self.MonArrayNum`))
  (`KismetArrayLibrary.Array_Remove` _monarraynum (`KismetArrayLibrary.Array_Find` _monarraynum ItemToFind)))

(fn `BP_Spawn_AutoGenFunc`)

(fn `SpawnNumber`
  (returns (OutputPin :type "/Game/_Dev/Monster_KHJ/BP_Monster Object Reference"))
  (bind _returnvalue (`|SpawnActorFromClass` "/Game/_Dev/Monster_KHJ/BP_Monster.BP_Monster_C" (`SceneComponent.K2_GetComponentToWorld` (`self.Arrow`)) "Undefined" "OverrideRootScale" null null))
  (return _returnvalue))

(fn `UserConstructionScript`)