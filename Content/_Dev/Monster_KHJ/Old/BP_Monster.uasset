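; Monster actor that travels along the level's BP_Spline toward an end point and takes damage, apparently for a wave-based game.
; A timeline drives spline position and rotation, while a GameState delegate supplies max HP and speed.
; Reaching BP_EndPoint updates the count, calls spawner pooling removal and resets position.
; Damage updates front and back HP bars; Tick hides the monster and disables collision when HP runs out.
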(event `self.ReceiveBeginPlay`
  (bind _returnvalue (`KismetMathLibrary.FTrunc` (`self.MonsterMaxHP`)))
  ;[1 1 1] 스플라인
  (bind _returnvalue_2 (`GameplayStatics.GetActorOfClass` "/Game/_Dev/Monster_KHJ/Old/BP_Spline.BP_Spline_C"))
  (set `self.BP_Spline_0` _returnvalue_2)
  (bind _returnvalue_3 (`GameplayStatics.GetActorOfClass` "/Game/_Dev/Monster_KHJ/Old/BP_EndPoint.BP_EndPoint_C"))
  (set `self. BP_EndPoint` _returnvalue_3)
  (`self.MoveTo`)
  (bind _asbp_game_state (cast `/Game/_Dev/Monster_KHJ/Old/BP_GameState` (`GameplayStatics.GetGameState`)))
  (set `self.BP_GameState` _asbp_game_state)
  (bind _returnvalue_4 (`GameplayStatics.GetActorOfClass` "/Game/_Dev/Monster_KHJ/Old/BP_Spawn.BP_Spawn_C"))
  (set `self.BP_Spawn` _returnvalue_4)
  (add `/Game/_Dev/Monster_KHJ/Old/BP_GameState.UpdateDT` (`self.BP_GameState`) (delegate `UpdateValue`))
  (`|ExecutionSequence`
    (:`then_0`
      (bind _ashp_bar (cast `/Game/_Dev/Character_CSH/Object/HpBar` (`WidgetComponent.GetUserWidgetObject` (`self.BackHPBar`))))
      (`/Game/_Dev/Character_CSH/Object/HpBar.CalHP` _ashp_bar 0 _returnvalue))
    (:`then_1`
      (bind _ashp_bar_2 (cast `/Game/_Dev/Character_CSH/Object/HpBar` (`WidgetComponent.GetUserWidgetObject` (`self.FrontHPBar`))))
      (`/Game/_Dev/Character_CSH/Object/HpBar.CalHP` _ashp_bar_2 0 _returnvalue))))

(event `UpdateValue`
  (params (MaxHP :type "Float (double-precision)") (MaxCount :type "Float (double-precision)") (Speed :type "Float (double-precision)"))
  (bind _output_get (set `self.MonsterMaxHP` MaxHP))
  (set `self.MonsterCurHP` _output_get)
  (set `self.Speed` Speed))

(event `MoveTo`
  ;[1 1 1] 스플라인상 움직임
  (`TimelineComponent.SetPlayRate` (`self.Move`) (`self.Speed`))
  (bind (_direction `_새_트랙_0`) (`Timeline|Move` :!via `PlayFromStart`)
    (:`Update`
      (`self.MoveToSpline` `_새_트랙_0`))))

(event `FollowSpline`
  ;[1 1 1] FollowSpline
  (if (and (`/Game/_Dev/Monster_KHJ/Old/BP_GameState.SpawnTimeBoolean` (`self.BP_GameState`)) (`/Game/_Dev/Monster_KHJ/Old/BP_Spawn.MaxArraySpawning` (`self.BP_Spawn`)))
    (`SceneComponent.SetVisibility` (`self.Capsule`) true false)
    (`SceneComponent.SetVisibility` (`self.SkeletalMesh`) true false)
    (`/Game/_Dev/Monster_KHJ/Old/BP_GameState.111111` (`self.BP_GameState`) self)))

(event `self.Capsule.OnComponentBeginOverlap`
  (params (OverlappedComponent :type "PrimitiveComponent Object Reference") (OtherActor :type "Actor Object Reference") (OtherComp :type "PrimitiveComponent Object Reference") (OtherBodyIndex :type Integer) (bFromSweep :type Boolean) (SweepResult :type "HitResult Structure (by ref)"))
  ;[1 1 1] Capsule BeginOverlap
  (`|ExecutionSequence`
    (:`then_0`
      (cast `/Game/_Dev/Monster_KHJ/Old/BP_EndPoint` OtherActor)
      (`SceneComponent.SetVisibility` (`self.Capsule`) false false)
      (`/Game/_Dev/Monster_KHJ/Old/BP_GameState.UpdateCount` (`self.BP_GameState`))
      (`/Game/_Dev/Monster_KHJ/Old/BP_Spawn.Pooling Remove` (`self.BP_Spawn`) self)
      (`self.InitialValue`)
      (`TimelineComponent.Stop` (`self.Move`)))))

(event `self.ReceiveAnyDamage`
  (params (Damage :type "Float (single-precision)") (DamageType :type "DamageType Object Reference") (InstigatedBy :type "Controller Object Reference") (DamageCauser :type "Actor Object Reference"))
  (bind _output_get (set `self.HP` (- (`self.HP`) Damage)))
  (`KismetSystemLibrary.PrintString` (`KismetStringLibrary.Conv_DoubleToString` _output_get))
  (set `self.MonsterCurHP` (- (`self.MonsterCurHP`) Damage))
  (`|ExecutionSequence`
    (:`then_0`
      (bind _ashp_bar (cast `/Game/_Dev/Character_CSH/Object/HpBar` (`WidgetComponent.GetUserWidgetObject` (`self.BackHPBar`))))
      (`/Game/_Dev/Character_CSH/Object/HpBar.CalHP` _ashp_bar (`KismetMathLibrary.FTrunc` (`self.MonsterCurHP`)) (`KismetMathLibrary.FTrunc` (`self.MonsterMaxHP`))))
    (:`then_1`
      (bind _ashp_bar_2 (cast `/Game/_Dev/Character_CSH/Object/HpBar` (`WidgetComponent.GetUserWidgetObject` (`self.FrontHPBar`))))
      (`/Game/_Dev/Character_CSH/Object/HpBar.CalHP` _ashp_bar_2 (`KismetMathLibrary.FTrunc` (`self.MonsterCurHP`)) (`KismetMathLibrary.FTrunc` (`self.MonsterMaxHP`))))))

(event `self.ReceiveTick`
  (params (DeltaSeconds :type "Float (single-precision)"))
  (if (<= (`self.HP`) 0.0)
    (`SceneComponent.SetVisibility` (`self.Capsule`) false false)
    (`SceneComponent.SetVisibility` (`self.SkeletalMesh`) false false)
    (`PrimitiveComponent.SetCollisionEnabled` (`self.Capsule`) "NoCollision")
    (`PrimitiveComponent.SetCollisionEnabled` (`self.SkeletalMesh`) "NoCollision")))

(fn `InitialValue`
  ;[1 1 1] 초기값 리셋
  (`self.K2_SetActorLocation` (`SplineComponent.GetLocationAtSplinePoint` (`/Game/_Dev/Monster_KHJ/Old/BP_Spline.Spline` (`self.BP_Spline_0`)) 35 "World")))

(fn `LevelUp`
  (returns (`Stage Monster Max HP` :type "Float (double-precision)") (`Stage Monster Max Count` :type "Float (double-precision)"))
  (bind (_stage_stage _stage_monstermaxhp _stage_monstermaxcount) (break `/Game/_Dev/Monster_KHJ/Old/ST_Max` (`self.Stage`)))
  (bind (_stage_stage_2 _stage_monstermaxhp_2 _stage_monstermaxcount_2) (break `/Game/_Dev/Monster_KHJ/Old/ST_Max` (`self.Stage`)))
  (bind (_stage_stage_3 _stage_monstermaxhp_3 _stage_monstermaxcount_3 _stage_monsterspeed) (break `/Game/_Dev/Monster_KHJ/Old/ST_Max` (`self.Stage`)))
  (bind (_stage_stage_4 _stage_monstermaxhp_4 _stage_monstermaxcount_4) (break `/Game/_Dev/Monster_KHJ/Old/ST_Max` (`self.Stage`)))
  (set `self.Stage` (make `/Game/_Dev/Monster_KHJ/Old/ST_Max` (+ _stage_stage_4 1) (* _stage_monstermaxhp_4 1.25) (* _stage_monstermaxcount_4 1.25)))
  (bind _result (`/Engine/EditorBlueprintResources/StandardMacros.IncrementInt` (`self.Count`))
    (:`  `
      (if (> _result 3)
        (set `self.Stage` (make `/Game/_Dev/Monster_KHJ/Old/ST_Max` _stage_stage_3 _stage_monstermaxhp_3 _stage_monstermaxcount_3 (+ _stage_monsterspeed 1.0)))
        (set `self.Count` 0)
        (return _stage_monstermaxhp_2 _stage_monstermaxcount_2)
        (else
          (return _stage_monstermaxhp _stage_monstermaxcount))))))

(fn `MoveToSpline`
  (params (Alpha :type "Float (double-precision)"))
  (bind _spline (`/Game/_Dev/Monster_KHJ/Old/BP_Spline.Spline` (`self.BP_Spline_0`)))
  (bind _returnvalue (`KismetMathLibrary.Lerp` 0.0 (`SplineComponent.GetSplineLength` (`/Game/_Dev/Monster_KHJ/Old/BP_Spline.Spline` (`self.BP_Spline_0`))) Alpha))
  (`self.K2_SetActorTransform` (`KismetMathLibrary.MakeTransform` (`SplineComponent.GetLocationAtDistanceAlongSpline` _spline _returnvalue "World") (`SplineComponent.GetRotationAtDistanceAlongSpline` _spline _returnvalue "World"))))

(fn `OnApplyDamage`
  (params (Damage :type "Float (double-precision)"))
  (if (> (`self.MonsterCurHP`) 0.0)
    (set `self.MonsterCurHP` (- (`self.MonsterCurHP`) Damage))
    (if (<= (`self.MonsterCurHP`) 0.0)
      _)))

(fn `UserConstructionScript`)