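; Game state prototype for monster stage progression, with a Tick timer that periodically raises a spawn flag.
; UpdateCount decrements the monster count and calls StageUp at zero, but StageUp is empty.
; StageUpdate scales stage stats, but its caller and the DT_Max/BP_Spawn setup are disconnected.
; BeginPlay only reads a DT_ddd row, and a custom event calls MoveTo after a recycle delay.
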(event `self.ReceiveBeginPlay`
  (bind _returnvalue (`|GetDataTableRow` "/Game/_Dev/Monster_KHJ/Old/DT_ddd.DT_ddd" (`KismetStringLibrary.Conv_StringToName` (`KismetStringLibrary.Conv_IntToString` (`self.RowName`))))
    (:`then`
      (set `self.아웃 행` _returnvalue))))

(event `self.ReceiveTick`
  (params (DeltaSeconds :type "Float (single-precision)"))
  (`self.SpawnTimeCondition` DeltaSeconds))

(event `UpdateCount`
  (bind _output_get (set `self.MonsterCount` (- (`self.MonsterCount`) 1.0)))
  (if (<= _output_get 0.0)
    (`self.StageUp`)
    (else
      (`KismetSystemLibrary.PrintString` "Stage Up Fail"))))

(event `StageUp`)

(event `111111`
  (params (NewParam :type "/Game/_Dev/Monster_KHJ/Old/BP_Monster Object Reference"))
  (`KismetSystemLibrary.PrintString` "Recycle Delay Start")
  (`KismetSystemLibrary.Delay` 2.0)
  (`/Game/_Dev/Monster_KHJ/Old/BP_Monster.MoveTo` NewParam))

(fn `NewFunction_0`)

(fn `SpawnTimeCondition`
  (params (A :type "Float (double-precision)"))
  (bind _output_get (set `self.CurrentTime` (+ A (`self.CurrentTime`))))
  (if (> _output_get (`self.DelayTime`))
    (set `self.SpawnTimeBoolean` true)
    (set `self.CurrentTime` 0.0)))

(fn `StageUpdate`
  (returns (`Stage Monster Max HP` :type "Float (double-precision)") (`Stage Monster Max Count` :type "Float (double-precision)") (`Main DT Monster Speed` :type "Float (double-precision)"))
  (bind (_maindt_stage _maindt_monstermaxhp _maindt_monstermaxcount _maindt_monsterspeed) (break `/Game/_Dev/Monster_KHJ/Old/ST_Max` (`self.MainDT`)))
  (bind (_maindt_stage_2 _maindt_monstermaxhp_2 _maindt_monstermaxcount_2 _maindt_monsterspeed_2) (break `/Game/_Dev/Monster_KHJ/Old/ST_Max` (`self.MainDT`)))
  (bind (_maindt_stage_3 _maindt_monstermaxhp_3 _maindt_monstermaxcount_3 _maindt_monsterspeed_3) (break `/Game/_Dev/Monster_KHJ/Old/ST_Max` (`self.MainDT`)))
  (bind (_maindt_stage_4 _maindt_monstermaxhp_4 _maindt_monstermaxcount_4) (break `/Game/_Dev/Monster_KHJ/Old/ST_Max` (`self.MainDT`)))
  (set `self.MainDT` (make `/Game/_Dev/Monster_KHJ/Old/ST_Max` (+ _maindt_stage_4 1) (* _maindt_monstermaxhp_4 1.25) (* _maindt_monstermaxcount_4 3.0)))
  (bind _result (`/Engine/EditorBlueprintResources/StandardMacros.IncrementInt` (`self.Count`))
    (:`  `
      (if (>= _result 2)
        (set `self.MainDT` (make `/Game/_Dev/Monster_KHJ/Old/ST_Max` _maindt_stage_3 _maindt_monstermaxhp_3 _maindt_monstermaxcount_3 (+ _maindt_monsterspeed_3 1.0)))
        (set `self.Count` 0)
        (return _maindt_monstermaxhp_2 _maindt_monstermaxcount_2 _maindt_monsterspeed_2)
        (else
          (return _maindt_monstermaxhp _maindt_monstermaxcount _maindt_monsterspeed))))))

(fn `UserConstructionScript`)