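; Reusable homing missile that damages its assigned target, hiding and resetting its Cube instead of being destroyed.
; While the Cube is visible, Tick restarts a timeline that eases it from its current transform toward the Target.
; Overlap with the target's capsule applies damage; that, an invalid target or the SetTimer timeout resets the Cube.
; Nothing here shows the Cube or assigns Target; debug prints and disconnected movement experiments remain.
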(event `self.ReceiveBeginPlay`
  (bind _cube (`self.Cube`))
  (`SceneComponent.SetVisibility` _cube false false)
  (`PrimitiveComponent.SetCollisionEnabled` _cube "NoCollision"))

(event `SetTimer`
  (`KismetSystemLibrary.K2_SetTimer` null "TimeOver" 0.5))

(event `self.ReceiveTick`
  (params (DeltaSeconds :type "Float (single-precision)"))
  (bind _cube (`self.Cube`))
  (bind _cube_2 (`self.Cube`))
  (if (`SceneComponent.IsVisible` (`self.Cube`))
    (`/Engine/EditorBlueprintResources/StandardMacros.IsValid` (`self.Target`)
      (:`Is Valid`
        (`KismetSystemLibrary.PrintString` "BeforeTimeline" true true (struct :`A` 1.0) 10.0)
        (bind (_direction `_새_트랙_0`) (`Timeline|타임라인_Attack` :!via `PlayFromStart` :!label _label)
          (:`Update`
            (`/Engine/EditorBlueprintResources/StandardMacros.IsValid` (`self.Target`)
              (:`Is Valid`
                (`SceneComponent.K2_SetWorldTransform` (`self.Cube`) (`KismetMathLibrary.MakeTransform` (.location (`|EaseFunction` "Linear" `_새_트랙_0` (`SceneComponent.K2_GetComponentToWorld` (`self.Cube`)) (`self.GetTransform` (`self.Target`)))) (.rotation (`|EaseFunction` "Linear" `_새_트랙_0` (`SceneComponent.K2_GetComponentToWorld` (`self.Cube`)) (`self.GetTransform` (`self.Target`))))) false false))
              (:`Is Not Valid`
                (`SceneComponent.SetVisibility` _cube false false)
                (`PrimitiveComponent.SetCollisionEnabled` _cube "NoCollision")
                (`SceneComponent.K2_SetRelativeLocation` (`self.Cube`) (0.0 0.0 0.0) false false))))))
      (:`Is Not Valid`
        (`KismetSystemLibrary.PrintString` "TargetNotVaild" true true (struct :`R` 1.0 :`B` 0.098177 :`A` 1.0) 10.0)
        (`SceneComponent.SetVisibility` _cube_2 false false)
        (`PrimitiveComponent.SetCollisionEnabled` _cube_2 "NoCollision")
        (`SceneComponent.K2_SetRelativeLocation` (`self.Cube`) (0.0 0.0 0.0) false false)))))

(event `StopCall`
  (goto _label :!via `Stop`))

(event `SetNewTime`
  (goto _label :!via `SetNewTime`))

(event `self.Cube.OnComponentBeginOverlap`
  (params (OverlappedComponent :type "PrimitiveComponent Object Reference") (OtherActor :type "Actor Object Reference") (OtherComp :type "PrimitiveComponent Object Reference") (OtherBodyIndex :type Integer) (bFromSweep :type Boolean) (SweepResult :type "HitResult Structure (by ref)"))
  (bind _cube (`self.Cube`))
  (bind _cube_2 (`self.Cube`))
  (bind _target (`self.Target`))
  (if (== OtherActor _target)
    (if (== (`Monster.Capsule` _target) OtherComp)
      (`GameplayStatics.ApplyDamage` _target (`self.Damage`))
      (`self.StopCall`)
      (set `self.Target` null)
      (`SceneComponent.SetVisibility` _cube_2 false false)
      (`PrimitiveComponent.SetCollisionEnabled` _cube_2 "NoCollision")
      (`SceneComponent.K2_SetRelativeLocation` _cube (0.0 0.0 0.0) false false)
      (`KismetSystemLibrary.PrintString` (`KismetStringLibrary.Conv_VectorToString` (`SceneComponent.RelativeLocation` _cube)) true true (struct :`R` 0.188449 :`G` 1.0 :`A` 1.0) 10.0)
      (`KismetSystemLibrary.K2_ClearTimer` null "TimeOver"))))

(event `self.Cube.OnComponentEndOverlap`
  (params (OverlappedComponent :type "PrimitiveComponent Object Reference") (OtherActor :type "Actor Object Reference") (OtherComp :type "PrimitiveComponent Object Reference") (OtherBodyIndex :type Integer)))

(fn `TimeOver`
  (bind _cube (`self.Cube`))
  (set `self.Target` null)
  (`SceneComponent.SetVisibility` _cube false false)
  (`PrimitiveComponent.SetCollisionEnabled` _cube "NoCollision")
  (`SceneComponent.K2_SetRelativeLocation` (`self.Cube`) (0.0 0.0 0.0) false false)
  (`self.SetNewTime`)
  (`KismetSystemLibrary.PrintString` "AAAAAAAAAAAAAAAAA" true true (struct :`R` 1.0 :`G` 0.010851 :`A` 1.0)))

(fn `UserConstructionScript`)