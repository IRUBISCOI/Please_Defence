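; BP_ExChar is a player Blueprint for placing summons on tower zones, with F toggling summon mode.
; While the mode is on, the Draw axis event traces from the follow camera through the mouse, showing the BeforeSummonzone preview on the hovered "Tower"-tagged BP_SummonZone.
; A left click repeats the trace, calls Summon on the hit zone and hides the cached zone's preview.
; Both traces draw debug lines.
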(event `Key|F`
  (params (Key :type "Key Structure"))
  (:`Pressed`
    (set `self.IsSummon` (not (`self.IsSummon`)))
    (if (not (`self.IsSummon`))
      (set `self.IsDraw` false))))

(event `InputAxis|Draw`
  (params (AxisValue :type "Float (single-precision)"))
  (bind (_worldlocation _worlddirection) (`PlayerController.DeprojectMousePositionToWorld` (`GameplayStatics.GetPlayerController` 0)))
  (if (`self.IsSummon`)
    (bind _outhit (`KismetSystemLibrary.LineTraceSingle` :`Start` (`SceneComponent.K2_GetComponentLocation` (`self.FollowCamera`)) :`End` (+ _worldlocation (* _worlddirection 1000.0)) :`TraceChannel` "TraceTypeQuery1" :`DrawDebugType` "ForDuration" :`TraceColor` (struct :`R` 1.0 :`G` 0.843707 :`A` 1.0) :`TraceHitColor` (struct :`G` 1.0 :`B` 0.884813 :`A` 1.0)))
    (bind (_bblockinghit _binitialoverlap _time _distance _location _impactpoint _normal _impactnormal _physmat _hitactor) (`GameplayStatics.BreakHitResult` _outhit))
    (`/Engine/EditorBlueprintResources/StandardMacros.IsValid` _hitactor
      (:`Is Valid`
        (if (`self.ActorHasTag` _hitactor "Tower")
          (`/Engine/EditorBlueprintResources/StandardMacros.IsValid` (`self.As BP Summon Zone`)
            (:`Is Valid`
              (`SceneComponent.SetVisibility` (`/Game/_Dev/Defencer_KHY/BP_SummonZone.BeforeSummonzone` (`self.As BP Summon Zone`)) false false)
              (bind _asbp_summon_zone (cast `/Game/_Dev/Defencer_KHY/BP_SummonZone` _hitactor))
              (bind _output_get (set `self.As BP Summon Zone` _asbp_summon_zone))
              (`SceneComponent.SetVisibility` (`/Game/_Dev/Defencer_KHY/BP_SummonZone.BeforeSummonzone` _output_get) true false))
            (:`Is Not Valid`
              (bind _asbp_summon_zone_2 (cast `/Game/_Dev/Defencer_KHY/BP_SummonZone` _hitactor))
              (bind _output_get_2 (set `self.As BP Summon Zone` _asbp_summon_zone_2))
              (`SceneComponent.SetVisibility` (`/Game/_Dev/Defencer_KHY/BP_SummonZone.BeforeSummonzone` _output_get_2) true false)))
          (else
            (`/Engine/EditorBlueprintResources/StandardMacros.IsValid` (`self.As BP Summon Zone`)
              (:`Is Valid`
                (`SceneComponent.SetVisibility` (`/Game/_Dev/Defencer_KHY/BP_SummonZone.BeforeSummonzone` (`self.As BP Summon Zone`)) false false)))))))))

(event `Key|LeftMouseButton`
  (params (Key :type "Key Structure"))
  (bind (_worldlocation _worlddirection) (`PlayerController.DeprojectMousePositionToWorld` (`GameplayStatics.GetPlayerController` 0)))
  (bind _beforesummonzone (`/Game/_Dev/Defencer_KHY/BP_SummonZone.BeforeSummonzone` (`self.As BP Summon Zone`)))
  (:`Pressed`
    (if (`self.IsSummon`)
      (bind _outhit (`KismetSystemLibrary.LineTraceSingle` :`Start` (`SceneComponent.K2_GetComponentLocation` (`self.FollowCamera`)) :`End` (+ _worldlocation (* _worlddirection 1000.0)) :`TraceChannel` "TraceTypeQuery1" :`DrawDebugType` "ForDuration" :`TraceColor` (struct :`G` 0.323312 :`B` 1.0 :`A` 1.0) :`TraceHitColor` (struct :`G` 1.0 :`B` 0.066493 :`A` 1.0)))
      (bind (_bblockinghit _binitialoverlap _time _distance _location _impactpoint _normal _impactnormal _physmat _hitactor) (`GameplayStatics.BreakHitResult` _outhit))
      (`/Engine/EditorBlueprintResources/StandardMacros.IsValid` _hitactor
        (:`Is Valid`
          (if (`self.ActorHasTag` _hitactor "Tower")
            (bind _asbp_summon_zone (cast `/Game/_Dev/Defencer_KHY/BP_SummonZone` _hitactor))
            (`/Game/_Dev/Defencer_KHY/BP_SummonZone.Summon` _asbp_summon_zone)
            (`/Engine/EditorBlueprintResources/StandardMacros.IsValid` _beforesummonzone
              (:`Is Valid`
                (`SceneComponent.SetVisibility` _beforesummonzone false false)))))))))

(fn `UserConstructionScript`)