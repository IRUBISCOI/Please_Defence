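; BP_BuffComponent is a buff component that currently only provides a particle effect at a stored location.
; StartAndLoopBuff caches damage, delay, particle template and location, but starts no timer or loop despite its name.
; Buff spawns that emitter without auto-destroy; its logic to add Damage to BP_Character and print the result is disconnected, and Delay is unused.
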(fn `Buff`
  (`GameplayStatics.SpawnEmitterAtLocation` (`self.Particle`) (`self.Location`) (struct) (1.0 1.0 1.0) false))

(fn `StartAndLoopBuff`
  (params (Damage :type "Float (double-precision)") (Delay :type "Float (double-precision)") (NewParam :type "ParticleSystem Object Reference") (Location :type "Vector Structure"))
  (set `self.Damage` Damage)
  (set `self.Delay` Delay)
  (set `self.Particle` NewParam)
  (set `self.Location` Location))