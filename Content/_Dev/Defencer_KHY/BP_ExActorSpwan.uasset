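; BP_ExActorSpwan is an example spawner actor that creates a batch of BP_ExEnemy actors at its own transform on BeginPlay.
; Each spawned enemy has its Sphere component hidden and is stored in an array, with names printed for debugging.
; After a delay, it loops through the array to reveal each Sphere and shift it along world X, then prints the names again.
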(event `self.ReceiveBeginPlay`
  (bind _newvar_1 (`self.NewVar_1`))
  (for _ (range 11)
    (bind _returnvalue (`|SpawnActorFromClass` "/Game/_Dev/Defencer_KHY/BP_ExEnemy.BP_ExEnemy_C" (`self.GetTransform`) "Undefined" "OverrideRootScale" null null))
    (bind _output_get (set `self.NewVar_0` _returnvalue))
    (`SceneComponent.SetVisibility` (`/Game/_Dev/Defencer_KHY/BP_ExEnemy.Sphere` _output_get) false false)
    (`KismetArrayLibrary.Array_Add` (`self.NewVar_1`) _output_get)
    (`KismetSystemLibrary.PrintString` (`KismetSystemLibrary.GetDisplayName` _output_get) true true (struct :`A` 1.0)))
  (for _array_element (`self.NewVar_1`)
    (`KismetSystemLibrary.PrintString` (`KismetSystemLibrary.GetDisplayName` _array_element) true true (struct :`R` 1.0 :`G` 1.0 :`B` 1.0 :`A` 1.0)))
  (`KismetSystemLibrary.Delay` 5.0)
  (for _array_element_2 _newvar_1
    (bind _sphere (`/Game/_Dev/Defencer_KHY/BP_ExEnemy.Sphere` _array_element_2))
    (`SceneComponent.SetVisibility` _sphere true false)
    (`SceneComponent.K2_AddWorldOffset` _sphere (100.0 0.0 0.0) false false))
  (for _ (range (+ (`KismetArrayLibrary.Array_Length` _newvar_1) 1))
    _)
  (for _array_element_3 _newvar_1
    (`KismetSystemLibrary.PrintString` (`KismetSystemLibrary.GetDisplayName` _array_element_3) true true (struct :`R` 1.0 :`B` 0.036115 :`A` 1.0))))

(fn `UserConstructionScript`)