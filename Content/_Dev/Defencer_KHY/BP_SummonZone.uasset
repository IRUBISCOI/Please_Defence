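; Dev tower summon zone child Blueprint that marks itself "Tower" with a pre-summon material, defers Summon to its parent, and prints target counts on Tick while IsOn.
; Attack cycles through a missile array, re-enabling visibility and collision; SetNormalTarget passes target, damage and transform to the missiles.
; Most older logic is disconnected: random DataTable-driven Normal/Skill/Buff tower setup, overlap-based nearest-monster targeting and missile pool spawning, leaving SetAttackArray empty.
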(event `self.Summon`
  (`parent.Summon`))

(event `self.ReceiveBeginPlay`
  (`PrimitiveComponent.SetMaterial` (`self.BeforeSummonZone`) 0 "/Game/_Dev/Defencer_KHY/M_DrawBeforeSummon.M_DrawBeforeSummon")
  (bind _output_get (set `self.tag` "Tower"))
  (set `self.Tags` (`|MakeArray` _output_get)))

(event `self.ReceiveTick`
  (params (DeltaSeconds :type "Float (single-precision)"))
  (bind _targetarr (`self.TargetArr`))
  (`parent.ReceiveTick` DeltaSeconds)
  (if (`self.IsOn`)
    (for _array_element _targetarr
      (`KismetSystemLibrary.PrintString` (`KismetStringLibrary.Concat_StrStr` "Monster:" (`KismetStringLibrary.Conv_IntToString` (`KismetArrayLibrary.Array_Length` _targetarr))) true true (struct :`R` 0.876576 :`G` 1.0 :`A` 1.0) 10.0))))

(fn `AAA`
  (set `self.DelayCheck` true))

(fn `Attack`
  (`/Engine/EditorBlueprintResources/StandardMacros.IsValid` (`self.Target`)
    (:`Is Valid`
      (if (> (`KismetMathLibrary.FTrunc` (`/Game/_Dev/Monster_KHJ/BP_Monster.HP` (`self.Target_0`))) 0)
        (if (>= (`self.ArrayNum`) 10)
          (set `self.ArrayNum` 0)
          (`self.MissileArrayReset`)
          (else
            (`self.MissileArrayReset`)))))))

(fn `ExSelectTower`)

(fn `MissileArrayReset`
  (bind _output (`|GetArrayItem` (`self.MissileArray`) (`self.ArrayNum`)))
  (`KismetSystemLibrary.PrintString` "MissileReset" true true (struct :`G` 1.0 :`B` 0.141677 :`A` 1.0) 10.0)
  (`/Engine/EditorBlueprintResources/StandardMacros.IsValid` _output
    (:`Is Valid`
      (bind _asbp_missile (cast `/Game/_Dev/Defencer_KHY/BP_Missile` _output))
      (bind _cube (`/Game/_Dev/Defencer_KHY/BP_Missile.Cube` _asbp_missile))
      (`SceneComponent.SetVisibility` _cube true false)
      (`PrimitiveComponent.SetCollisionEnabled` _cube "QueryAndPhysics")
      (set `self.ArrayNum` (+ (`self.ArrayNum`) 1))
      (`KismetSystemLibrary.PrintString` "IsMissile" true true (struct :`R` 1.0 :`B` 0.050545 :`A` 1.0) 100.0))))

(fn `SelectTarget`
  (set `self.Target_0` (`|GetArrayItem` (`self.As BP Monster`) (`self.MonsterNum`))))

(fn `SetAttackArray`)

(fn `SetNormalTarget`
  (for _array_element (`self.MisslieArray`)
    (set `/Game/_Dev/Defencer_KHY/BP_Missile.Target` (`self.Target`) _array_element)
    (set `/Game/_Dev/Defencer_KHY/BP_Missile.Damage` (`.Damage` (break `ST_NormalTower` (`self.NormalTower`))) _array_element)
    (set `/Game/_Dev/Defencer_KHY/BP_Missile.Transform` (`SceneComponent.K2_GetComponentToWorld` (`self.Tower`)) _array_element)))

(fn `Settimer`
  (`KismetSystemLibrary.PrintString` (`KismetSystemLibrary.GetDisplayName` (`self.Target`)) true true (struct :`R` 0.638761 :`B` 1.0 :`A` 1.0) 0.1))

(fn `UserConstructionScript`)