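; BP_SkillComponent is a skill component that stores skill settings and fires an active skill on a single target.
; SettingSkill and SetTarget supply the data, with range and distance stored but unused here.
; ActiveSkill debug-prints the target's location, then, if a particle is set, spawns it there enlarged and applies damage immediately.
; A function-name timer calls ClearEmitter to destroy the effect just before the skill delay elapses.
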(fn `Active Skill`
  (bind _loaction (`self.Loaction`))
  (bind _particle (`self.particle`))
  (`/Engine/EditorBlueprintResources/StandardMacros.IsValid` (`self.Target`)
    (:`Is Valid`
      (set `self.Loaction` (`Actor.K2_GetActorLocation` (`self.Target`)))
      (`KismetSystemLibrary.PrintString` (`KismetStringLibrary.Conv_VectorToString` _loaction) true true (struct :`R` 1.0 :`G` 1.0 :`B` 1.0 :`A` 1.0) 10.0)
      (`/Engine/EditorBlueprintResources/StandardMacros.IsValid` _particle
        (:`Is Valid`
          (bind _returnvalue (`GameplayStatics.SpawnEmitterAtLocation` _particle _loaction (struct) (10.0 10.0 10.0)))
          (set `self.SettingEmitter` _returnvalue)
          (`GameplayStatics.ApplyDamage` (`self.Target`) (`self.Damage`))
          (`KismetSystemLibrary.K2_SetTimer` null "ClearEmitter" (- (`self.Delay`) 0.1)))))))

(fn `ClearEmitter`
  (bind _settingemitter (`self.SettingEmitter`))
  (`/Engine/EditorBlueprintResources/StandardMacros.IsValid` _settingemitter
    (:`Is Valid`
      (`self.K2_DestroyComponent` _settingemitter)
      (`KismetSystemLibrary.K2_ClearTimer` null "ClearEmitter"))))

(fn `SetTarget`
  (params (Target :type "Actor Object Reference"))
  (set `self.Target` Target))

(fn `SettingSkill`
  (params (Rannge :type "Float (double-precision)") (Damage :type "Float (double-precision)") (Delay :type "Float (double-precision)") (Distance :type "Float (double-precision)") (Particle :type "ParticleSystem Object Reference") (Location :type "Vector Structure"))
  (set `self.Rannge` Rannge)
  (set `self.Damage` Damage)
  (set `self.Delay` Delay)
  (set `self.Distance` Distance)
  (set `self.particle` Particle)
  (set `self.Loaction` Location))